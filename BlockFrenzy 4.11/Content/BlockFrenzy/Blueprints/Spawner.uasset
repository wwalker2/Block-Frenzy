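; Spawner actor for BlockFrenzy that places regular and special blocks at random points inside its Box component.
; SpawnBlocks and SpecialBlockSpawn each count live actors of their class and spawn one more only while under MaxBlocks or MaxSpecialBlocks.
; Neither event is triggered within this Blueprint, as BeginPlay and Tick are unused, so timing comes from outside callers.
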(event `SpawnBlocks`
  (bind _box (`self.Box`))
  (bind _outactors (`GameplayStatics.GetAllActorsOfClass` "/Game/BlockFrenzy/Blueprints/TargetBlock.TargetBlock_C"))
  (if (< (`KismetArrayLibrary.Array_Length` _outactors) (`self.MaxBlocks`))
    (`|SpawnActorFromClass` "/Game/BlockFrenzy/Blueprints/TargetBlock.TargetBlock_C" (`KismetMathLibrary.Conv_VectorToTransform` (`KismetMathLibrary.RandomPointInBoundingBox` (`SceneComponent.K2_GetComponentLocation` _box) (`BoxComponent.GetScaledBoxExtent` _box))) "Undefined" "OverrideRootScale")))

(event `self.ReceiveBeginPlay`)

(event `self.ReceiveActorBeginOverlap`
  (params (OtherActor :type "Actor Object Reference")))

(event `self.ReceiveTick`
  (params (DeltaSeconds :type "Float (single-precision)")))

(event `SpecialBlockSpawn`
  (bind _box (`self.Box`))
  (bind _outactors (`GameplayStatics.GetAllActorsOfClass` "/Game/BlockFrenzy/Blueprints/SpecialBlock.SpecialBlock_C"))
  (if (< (`KismetArrayLibrary.Array_Length` _outactors) (`self.MaxSpecialBlocks`))
    (`|SpawnActorFromClass` "/Game/BlockFrenzy/Blueprints/SpecialBlock.SpecialBlock_C" (`KismetMathLibrary.Conv_VectorToTransform` (`KismetMathLibrary.RandomPointInBoundingBox` (`SceneComponent.K2_GetComponentLocation` _box) (`BoxComponent.GetScaledBoxExtent` _box))) "Undefined" "OverrideRootScale")))

(fn `UserConstructionScript`)