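; TargetBlock is a shootable, destructible target in Block Frenzy that awards a point to the player.
; When a FirstPersonProjectile hits its Destructible component, it applies point damage to the hit actor and increments the score on BlockFrenzyMode.
; It destroys itself four seconds after a hit, or when a five-second Delay started from Tick expires, whichever comes first.
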(event `self.ReceiveTick`
  (params (DeltaSeconds :type "Float (single-precision)"))
  (`KismetSystemLibrary.Delay` 5.0)
  (`self.K2_DestroyActor`))

(event `self.Destructible.OnComponentHit`
  (params (HitComponent :type "PrimitiveComponent Object Reference") (OtherActor :type "Actor Object Reference") (OtherComp :type "PrimitiveComponent Object Reference") (NormalImpulse :type "Vector Structure") (Hit :type "HitResult Structure (by ref)"))
  (bind (_bblockinghit _binitialoverlap _time _location _impactpoint _normal _impactnormal _physmat _hitactor) (`GameplayStatics.BreakHitResult` Hit))
  (bind _asfirst_person_projectile (cast `/Game/FirstPersonBP/Blueprints/FirstPersonProjectile` OtherActor))
  (`GameplayStatics.ApplyPointDamage` _hitactor 100.0 _impactpoint Hit null _asfirst_person_projectile "/Script/Engine.DamageType")
  (bind _asblock_frenzy_mode (cast `/Game/BlockFrenzy/Blueprints/BlockFrenzyMode` (`GameplayStatics.GetGameMode`)))
  (`/Game/BlockFrenzy/Blueprints/BlockFrenzyMode.IncrementScore` _asblock_frenzy_mode 1)
  (`KismetSystemLibrary.Delay` 4.0)
  (`self.K2_DestroyActor`))

(fn `UserConstructionScript`)