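; BlockFrenzyMode runs a timed BlockFrenzy round, tracking score and counting down to the GameOver level.
; On BeginPlay it finds the first Spawner actor, starts looping timers that call its normal and special block spawn functions at per-second rates, and adds the HUD widget.
; Tick decrements the remaining Time and opens GameOver at zero, while the IncrementScore event adds to Score.
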(event `self.ReceiveBeginPlay`
  (`|ExecutionSequence`
    (:`then_0`
      (bind _outactors (`GameplayStatics.GetAllActorsOfClass` "/Game/BlockFrenzy/Blueprints/Spawner.Spawner_C"))
      (bind _output_get (set `self.Spawner` (`KismetArrayLibrary.Array_Get` _outactors)))
      (`KismetSystemLibrary.K2_SetTimer` _output_get "SpawnBlocks" (/ 1.0 (`self.BlocksPerSec`)) true))
    (:`then_1`
      (`KismetSystemLibrary.K2_SetTimer` (`self.Spawner`) "SpecialBlockSpawn" (/ 1.0 (`self.SPBlocksPerSec`)) true))
    (:`then_2`
      (bind _returnvalue (`|CreateWidget` "/Game/BlockFrenzy/Blueprints/HUD.HUD_C"))
      (`UserWidget.AddToViewport` _returnvalue 0))))

(event `IncrementScore`
  (params (DeltaScore :type Integer))
  (set `self.Score` (+ DeltaScore (`self.Score`))))

(event `self.ReceiveTick`
  (params (DeltaSeconds :type "Float (single-precision)"))
  (bind _output_get (set `self.Time` (- (`self.Time`) DeltaSeconds)))
  (if (<= _output_get 0.0)
    (`GameplayStatics.OpenLevel` "GameOver")))

(fn `UserConstructionScript`)