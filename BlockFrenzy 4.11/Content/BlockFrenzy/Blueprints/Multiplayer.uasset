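; Multiplayer Blueprint that adds a local player in Block Frenzy.
; On BeginPlay it creates a player with controller ID 1 and pawn spawning enabled, then casts that player's pawn to FirstPersonCharacter with no further action.
; An unconnected leftover chain would create a player, manually spawn a FirstPersonCharacter and possess it, but never runs.
; Tick and the construction script only call their parents.
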(event `self.ReceiveBeginPlay`
  (`parent.ReceiveBeginPlay`)
  (bind _returnvalue (`GameplayStatics.CreatePlayer` 1))
  (cast `/Game/FirstPersonBP/Blueprints/FirstPersonCharacter` (`Controller.K2_GetPawn` _returnvalue)))

(event `self.ReceiveTick`
  (params (DeltaSeconds :type "Float (single-precision)"))
  (`parent.ReceiveTick` 0.0))

(fn `UserConstructionScript`
  (`parent.UserConstructionScript`))